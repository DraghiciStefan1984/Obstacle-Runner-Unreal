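; Player controller that drives MyCharacter through movement, look, jump and pause input.
; BeginPlay caches the player character cast to MyCharacter, and input events forward to it.
; Move axes add movement along the forward and right vectors of the control rotation, and look axes add pitch and yaw.
; The Pause action toggles the game's paused state.
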(event `self.ReceiveBeginPlay`
  (bind _asmy_character (cast `/Game/Blueprints/MyCharacter` (`GameplayStatics.GetPlayerCharacter` 0)))
  (set `self.MyCharacter` _asmy_character))

(event `InputAction|Jump`
  (params (Key :type "Key Structure"))
  (:`Pressed`
    (`Character.Jump` (`self.MyCharacter`))))

(event `InputAxis|MoveForwardBackward`
  (params (AxisValue :type "Float (single-precision)"))
  (bind _mycharacter (`self.MyCharacter`))
  (`Pawn.AddMovementInput` _mycharacter (`KismetMathLibrary.GetForwardVector` (`Pawn.GetControlRotation` _mycharacter)) AxisValue false))

(event `InputAxis|LookUpDown`
  (params (AxisValue :type "Float (single-precision)"))
  (`Pawn.AddControllerPitchInput` (`self.MyCharacter`) AxisValue))

(event `InputAxis|MoveRightLeft`
  (params (AxisValue :type "Float (single-precision)"))
  (bind _mycharacter (`self.MyCharacter`))
  (`Pawn.AddMovementInput` _mycharacter (`KismetMathLibrary.GetRightVector` (`Pawn.GetControlRotation` _mycharacter)) AxisValue false))

(event `InputAxis|LookLeftRight`
  (params (AxisValue :type "Float (single-precision)"))
  (`Pawn.AddControllerYawInput` (`self.MyCharacter`) AxisValue))

(event `InputAction|Pause` :paused true
  (params (Key :type "Key Structure"))
  (:`Pressed`
    (if (`GameplayStatics.IsGamePaused`)
      (`GameplayStatics.SetGamePaused` false)
      (else
        (`GameplayStatics.SetGamePaused` true)))))

(fn `UserConstructionScript`)