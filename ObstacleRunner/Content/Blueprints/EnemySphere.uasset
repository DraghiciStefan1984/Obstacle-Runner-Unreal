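; EnemySphere is a moving hazard actor that damages the player character on contact.
; On BeginPlay it stores its start location and plays a timeline that offsets it from that point each update, without sweeping.
; A UseXMovement flag selects whether the timeline's X or Y movement track drives the offset.
; Beginning an overlap with MyCharacter applies a small fixed amount of damage.
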(event `self.ReceiveBeginPlay`
  (bind _output_get (set `self.InitialEnemyLocation` (`self.K2_GetActorLocation`)))
  (bind (_direction _xmovement _ymovement) (`Timeline|EnemySphereTimeline`)
    (:`Update`
      (if (`self.UseXMovement`)
        (`self.K2_SetActorLocation` (+ _xmovement _output_get))
        (else
          (`self.K2_SetActorLocation` (+ _ymovement _output_get)))))))

(event `self.ReceiveActorBeginOverlap`
  (params (OtherActor :type "Actor Object Reference"))
  (bind _asmy_character (cast `/Game/Blueprints/MyCharacter` OtherActor))
  (`GameplayStatics.ApplyDamage` _asmy_character 0.2))

(fn `UserConstructionScript`)