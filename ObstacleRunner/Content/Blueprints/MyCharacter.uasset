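; MyCharacter is the character Blueprint that handles health, damage feedback and game over.
; BeginPlay creates and displays the HUD widget, and creates a pause menu widget that it stores without displaying.
; Damage passes through a DoOnce that resets after two short delays, giving brief invulnerability while a damage-tint flag pulses.
; When health runs out, game over is triggered and the GameOver event quits the game.
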(event `self.ReceiveBeginPlay`
  (bind _returnvalue (`|CreateWidget` "/Game/Blueprints/HUD_BP.HUD_BP_C"))
  (bind _output_get (set `self.HudReference` _returnvalue))
  (`UserWidget.AddToViewport` _output_get 0)
  (bind _returnvalue_2 (`|CreateWidget` "/Game/Blueprints/PauseMenu_BP.PauseMenu_BP_C"))
  (set `self.PauseMenuReference` _returnvalue_2))

(event `Event Game Over`
  (`KismetSystemLibrary.QuitGame` null "Quit"))

(event `self.ReceiveAnyDamage`
  (params (Damage :type "Float (single-precision)") (DamageType :type "DamageType Object Reference") (InstigatedBy :type "Controller Object Reference") (DamageCauser :type "Actor Object Reference"))
  (`/Engine/EditorBlueprintResources/StandardMacros.DoOnce` false :!label _label
    (:`Completed`
      (bind _output_get (set `self.Health` (- (`self.Health`) Damage)))
      (if (<= _output_get 0.0)
        (`self.Event Game Over`)
        (else
          (set `self.ShowDamageTint` true)
          (`KismetSystemLibrary.Delay` 0.3)
          (set `self.ShowDamageTint` false)
          (`KismetSystemLibrary.Delay` 0.2)
          (goto _label :!via `Reset`))))))

(fn `UserConstructionScript`)